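; Main character HUD that creates and holds references to the game's UI widgets: main, pause, options, connection, respawn, clue system, puzzle and boss dialogue screens.
; On BeginPlay it creates every widget up front, stores each in a variable, adds all to the viewport and sets them hidden.
; It then loads the saved game user settings; the HUD itself has no logic for showing the widgets.
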(event `self.ReceiveBeginPlay`
  ;[1 1 1] Initialize
  (bind _returnvalue (`|CreateWidget` "/Game/UI/InGameUI/PicturePuzzle/WBP_PuzzleWidget.WBP_PuzzleWidget_C"))
  (bind _output_get (set `self.wbp_PuzzleWidgetRef` _returnvalue))
  (bind _returnvalue_2 (`|CreateWidget` "/Game/UI/InGameUI/Respawn/WBP_Respawn.WBP_Respawn_C"))
  (bind _output_get_2 (set `self.wbp_RespawnRef` _returnvalue_2))
  (bind _returnvalue_3 (`|CreateWidget` "/Game/UI/InGameUI/Dialogue/WBP_ClueSystem.WBP_ClueSystem_C"))
  (bind _output_get_3 (set `self.wbp_ClueSystemRef` _returnvalue_3))
  (bind _returnvalue_4 (`|CreateWidget` "/Game/UI/InGameUI/Dialogue/WBP_DialogueBoss.WBP_DialogueBoss_C"))
  (bind _output_get_4 (set `self.wbp_DialogueBossRef` _returnvalue_4))
  (bind _returnvalue_5 (`|CreateWidget` "/Game/UI/InGameUI/Dialogue/WBP_DialogueBoss2.WBP_DialogueBoss2_C"))
  (bind _output_get_5 (set `self.wbp_DialogueBoss2Ref` _returnvalue_5))
  (bind _returnvalue_6 (`|CreateWidget` "/Game/UI/InGameUI/DoorPuzzle/WBP_PuzzleMain.WBP_PuzzleMain_C"))
  (bind _output_get_6 (set `self.wbp_DoorPuzzleRef` _returnvalue_6))
  (bind _returnvalue_7 (`|CreateWidget` "/Game/UI/InGameUI/WBP_MainUI.WBP_MainUI_C"))
  (bind _output_get_7 (set `self.wbp_MainRef` _returnvalue_7))
  (bind _returnvalue_8 (`|CreateWidget` "/Game/UI/Menu/OptionMenu/WBP_OptionMenu.WBP_OptionMenu_C"))
  (bind _output_get_8 (set `self.wbp_OptionRef` _returnvalue_8))
  (bind _returnvalue_9 (`|CreateWidget` "/Game/UI/InGameUI/WBP_PauseUI.WBP_PauseUI_C"))
  (bind _output_get_9 (set `self.wbp_PauseRef` _returnvalue_9))
  (bind _returnvalue_10 (`|CreateWidget` "/Game/UI/InGameUI/Connection/WBP_Connection.WBP_Connection_C"))
  (bind _output_get_10 (set `self.wbp_ConnectionRef` _returnvalue_10))
  (`UserWidget.AddToViewport` _output_get_10 0)
  (`UserWidget.AddToViewport` _output_get_9 0)
  (`UserWidget.AddToViewport` _output_get_7 0)
  (`UserWidget.AddToViewport` _output_get_8 0)
  (`UserWidget.AddToViewport` _output_get_6 0)
  (`UserWidget.AddToViewport` _output_get_4 0)
  (`UserWidget.AddToViewport` _output_get_5 0)
  (`UserWidget.AddToViewport` _output_get_3 0)
  (`UserWidget.AddToViewport` _output_get_2 0)
  (`UserWidget.AddToViewport` _output_get 0)
  (`Widget.SetVisibility` _output_get_7 "Hidden")
  (`Widget.SetVisibility` _output_get_9 "Hidden")
  (`Widget.SetVisibility` _output_get_10 "Hidden")
  (`Widget.SetVisibility` _output_get_8 "Hidden")
  (`Widget.SetVisibility` _output_get_6 "Hidden")
  (`Widget.SetVisibility` _output_get_4 "Hidden")
  (`Widget.SetVisibility` _output_get_5 "Hidden")
  (`Widget.SetVisibility` _output_get_3 "Hidden")
  (`Widget.SetVisibility` _output_get_2 "Hidden")
  (`Widget.SetVisibility` _output_get "Hidden")
  (bind _returnvalue_11 (`GameUserSettings.GetGameUserSettings`))
  (`GameUserSettings.LoadSettings` _returnvalue_11 false))

(fn `UserConstructionScript`)