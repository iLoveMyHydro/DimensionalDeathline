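; BP_HUDMenu is a menu HUD that sets up the main menu screens when play begins.
; It creates main menu, options and credits widgets and adds all three to the viewport, showing only the main menu and hiding the others.
; A fade widget sits above them at a higher Z-order and is removed after a short delay.
; References to each widget are stored in variables.
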(event `self.ReceiveBeginPlay`
  (bind _returnvalue (`|CreateWidget` "/Game/UI/Menu/MainMenu/WBP_fade.WBP_fade_C"))
  (bind _output_get (set `self.wbp_FadeRef` _returnvalue))
  (bind _returnvalue_2 (`|CreateWidget` "/Game/UI/Menu/MainMenu/WBP_MainMenu.WBP_MainMenu_C"))
  (bind _output_get_2 (set `self.wbp_MainRef` _returnvalue_2))
  (bind _returnvalue_3 (`|CreateWidget` "/Game/UI/Menu/CreditsMenu/WBP_CreditsMenuFix.WBP_CreditsMenuFix_C"))
  (bind _output_get_3 (set `self.wbp_CreditsRef` _returnvalue_3))
  (bind _returnvalue_4 (`|CreateWidget` "/Game/UI/Menu/OptionMenu/WBP_OptionMenu.WBP_OptionMenu_C"))
  (bind _output_get_4 (set `self.wbp_OptionRef` _returnvalue_4))
  (`UserWidget.AddToViewport` _output_get_2 0)
  (`UserWidget.AddToViewport` _output_get_4 0)
  (`UserWidget.AddToViewport` _returnvalue_3 0)
  (`Widget.SetVisibility` _returnvalue_2 "Visible")
  (`Widget.SetVisibility` _returnvalue_4 "Hidden")
  (`Widget.SetVisibility` _output_get_3 "Hidden")
  (`UserWidget.AddToViewport` _output_get 1)
  (`KismetSystemLibrary.Delay` 2.0)
  (`Widget.RemoveFromParent` _output_get))

(fn `UserConstructionScript`)