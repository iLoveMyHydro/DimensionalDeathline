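; Dialogue decorator that plays Zaq's flashback cutscene when executed.
; It stops the jukebox music, hides the mouse cursor, plays the flashback sound through the BP_ZaqAudio actor and shows the WBP_VideoZaq widget.
; A fixed Delay, rather than a playback-finished event, times the cutscene's end, then the widget is removed, the cursor returns and the jukebox plays again from the start.
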(event `self.ExecuteDecorator`
  (bind _returnvalue (`GameplayStatics.GetActorOfClass` "/Game/Blueprint/InventorySystem/Items/BP_jukebox.BP_jukebox_C"))
  (`AudioComponent.Stop` (`/Game/Blueprint/InventorySystem/Items/BP_jukebox.Audio` _returnvalue))
  (set `PlayerController.bShowMouseCursor` false (`GameplayStatics.GetPlayerController` 0))
  (bind _returnvalue_2 (`|CreateWidget` "/Game/VFX/WBP_VideoZaq.WBP_VideoZaq_C"))
  (bind _returnvalue_3 (`GameplayStatics.GetActorOfClass` "/Game/VFX/BP_ZaqAudio.BP_ZaqAudio_C"))
  (bind _audio (`/Game/VFX/BP_ZaqAudio.Audio` _returnvalue_3))
  (`AudioComponent.SetSound` _audio "/Game/Audio/SFX/SFX_Cutscene_Flashback.SFX_Cutscene_Flashback")
  (`AudioComponent.Play` _audio 0.0)
  (`UserWidget.AddToViewport` _returnvalue_2 0)
  (`KismetSystemLibrary.Delay` 107.0)
  (`Widget.RemoveFromParent` _returnvalue_2)
  (set `PlayerController.bShowMouseCursor` true (`GameplayStatics.GetPlayerController` 0))
  (bind _returnvalue_4 (`GameplayStatics.GetActorOfClass` "/Game/Blueprint/InventorySystem/Items/BP_jukebox.BP_jukebox_C"))
  (`AudioComponent.Play` (`/Game/Blueprint/InventorySystem/Items/BP_jukebox.Audio` _returnvalue_4) 0.0))