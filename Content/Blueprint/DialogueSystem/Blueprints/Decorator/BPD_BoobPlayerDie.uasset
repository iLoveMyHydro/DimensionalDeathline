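; Dialogue decorator that handles the player dying through the first wagon event during a dialogue.
; On execution it sets the wagon 01 death flag on BP_GameInstance.
; On cleanup it shows the mouse cursor, makes the respawn widget held by BP_MainHUD visible and switches the player controller to UI-only input.
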(event `self.ExecuteDecorator`
  (bind _asbp_game_instance (cast `/Game/Blueprint/GameInstance/BP_GameInstance` (`GameplayStatics.GetGameInstance`)))
  (set `/Game/Blueprint/GameInstance/BP_GameInstance.b_PlayerDiedViaWagon01` true _asbp_game_instance))

(event `self.CleanupDecorator`
  (set `PlayerController.bShowMouseCursor` true (`GameplayStatics.GetPlayerController` 0))
  (bind _asbp_main_hud (cast `/Game/Characters/MainCharacter/HUD/BP_MainHUD` (`PlayerController.GetHUD` (`GameplayStatics.GetPlayerController` 0))))
  (`Widget.SetVisibility` (`/Game/Characters/MainCharacter/HUD/BP_MainHUD.wbp_RespawnRef` _asbp_main_hud) "Visible")
  (`WidgetBlueprintLibrary.SetInputMode_UIOnlyEx` (`GameplayStatics.GetPlayerController` 0) null))