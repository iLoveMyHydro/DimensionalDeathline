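; BP_SwitchCamera is a dialogue system decorator that switches the player's view to a designated camera and restores it afterward.
; On execute, it async-loads a referenced CameraActor and blends player controller 0's view target to it using cubic blending.
; On cleanup, it blends back to the player's BP_DialogMainCharacter with the same configurable blend time.
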(event `self.ExecuteDecorator`
  (bind _object (`|LoadAsset` (`self.CameraActorRef`))
    (:`Completed`
      (bind _ascamera_actor (cast `CameraActor` _object))
      (`PlayerController.SetViewTargetWithBlend` (`GameplayStatics.GetPlayerController` 0) _ascamera_actor (`self.f_BlendTime`) "VTBlend_Cubic" 0.0 false))))

(event `self.CleanupDecorator`
  (bind _asbp_dialog_main_character (cast `/Game/Characters/MainCharacter/BP_DialogMainCharacter` (`GameplayStatics.GetPlayerCharacter` 0)))
  (`PlayerController.SetViewTargetWithBlend` (`GameplayStatics.GetPlayerController` 0) _asbp_dialog_main_character (`self.f_BlendTime`) "VTBlend_Cubic" 0.0 false))