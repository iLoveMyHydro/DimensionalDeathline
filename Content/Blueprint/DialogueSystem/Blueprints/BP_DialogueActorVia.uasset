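; BP_DialogueActorVia is the NPC actor for Via, who talks to the player through the Mountea Dialogue system.
; Participant commands Idle, Talk and Kill each swap her skeletal animation and the material on a plane.
; StartDialogue checks GameInstance progress flags and a local once-only flag to start the initial, second lobby or wagon dialogue through the player character.
; Its sequenced checks are not exclusive, so one call can trigger several starts.
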(event `self.ReceiveBeginPlay`
  (add `MounteaDialogueParticipant.ParticipantCommandRequested` (`self.NPC_MounteaDialogueParticipant`) (delegate `Idle`))
  (add `MounteaDialogueParticipant.ParticipantCommandRequested` (`self.NPC_MounteaDialogueParticipant`) (delegate `Talk`))
  (add `MounteaDialogueParticipant.ParticipantCommandRequested` (`self.NPC_MounteaDialogueParticipant`) (delegate `Kill`)))

(event `Idle`
  (params (Command :type String) (OptionalPayload :type "Object Object Reference"))
  (if (== Command "Idle")
    (`SkeletalMeshComponent.PlayAnimation` (`self.SkeletalMesh`) "/Game/Characters/via/Animations/Via_Idle_Anim.Via_Idle_Anim" true)
    (`PrimitiveComponent.SetMaterial` (`self.Plane`) 0 "/Game/Characters/via/Materials/Via_Idle.Via_Idle")))

(event `Talk`
  (params (Command :type String) (OptionalPayload :type "Object Object Reference"))
  (if (== Command "Talk")
    (`SkeletalMeshComponent.PlayAnimation` (`self.SkeletalMesh`) "/Game/Characters/via/Animations/Via_Talk_Anim.Via_Talk_Anim" true)
    (`PrimitiveComponent.SetMaterial` (`self.Plane`) 0 "/Game/Characters/via/Materials/Via_Talk.Via_Talk")))

(event `Kill`
  (params (Command :type String) (OptionalPayload :type "Object Object Reference"))
  (if (== Command "Kill")
    (`SkeletalMeshComponent.PlayAnimation` (`self.SkeletalMesh`) "/Game/Characters/via/Animations/Via_Kill_Anim.Via_Kill_Anim" false)
    (`PrimitiveComponent.SetMaterial` (`self.Plane`) 0 "/Game/Characters/via/Materials/Via_Kill.Via_Kill")))

(event `self.StartDialogue`
  (bind _npc_mounteadialogueparticipant (`self.NPC_MounteaDialogueParticipant`))
  (`/Engine/EditorBlueprintResources/StandardMacros.Can Execute Cosmetic Events`
    (:`True`
      (`/Engine/EditorBlueprintResources/StandardMacros.IsValid` (`self.GetComponentByClass` "/Script/MounteaDialogueSystem.MounteaDialogueParticipant")
        (:`Is Valid`
          (`|ExecutionSequence`
            (:`then_0`
              (bind _asbp_game_instance (cast `/Game/Blueprint/GameInstance/BP_GameInstance` (`GameplayStatics.GetGameInstance`)))
              (if (not (`/Game/Blueprint/GameInstance/BP_GameInstance.b_TalkedWithVia` _asbp_game_instance))
                (bind _asbp_dialog_main_character (cast `/Game/Characters/MainCharacter/BP_DialogMainCharacter` (`GameplayStatics.GetPlayerCharacter` 0)))
                (`/MounteaDialogueSystem/Blueprints/Core/BP_Dialogue_Character.Start Dialogue from Player` _asbp_dialog_main_character self)
                (bind _asbp_game_instance_2 (cast `/Game/Blueprint/GameInstance/BP_GameInstance` (`GameplayStatics.GetGameInstance`)))
                (set `/Game/Blueprint/GameInstance/BP_GameInstance.b_TalkedWithVia` true _asbp_game_instance_2)))
            (:`then_1`
              (bind _asbp_game_instance_3 (cast `/Game/Blueprint/GameInstance/BP_GameInstance` (`GameplayStatics.GetGameInstance`)))
              (if (`/Game/Blueprint/GameInstance/BP_GameInstance.b_TalkedWithVia` _asbp_game_instance_3)
                (if (not (`self.b_TalkedWithVia2`))
                  (`MounteaDialogueParticipantInterface.SetDialogueGraph` _npc_mounteadialogueparticipant "/Game/Blueprint/DialogueSystem/Dialogues/Via/Lobby/MDT_Via_Lobby_2.MDT_Via_Lobby_2")
                  (bind _asbp_dialog_main_character_2 (cast `/Game/Characters/MainCharacter/BP_DialogMainCharacter` (`GameplayStatics.GetPlayerCharacter` 0)))
                  (`/MounteaDialogueSystem/Blueprints/Core/BP_Dialogue_Character.Start Dialogue from Player` _asbp_dialog_main_character_2 self)
                  (set `self.b_TalkedWithVia2` true))))
            (:`then_2`
              (bind _asbp_game_instance_4 (cast `/Game/Blueprint/GameInstance/BP_GameInstance` (`GameplayStatics.GetGameInstance`)))
              (if (`/Game/Blueprint/GameInstance/BP_GameInstance.b_GotVIACharger` _asbp_game_instance_4)
                (`MounteaDialogueParticipantInterface.SetDialogueGraph` _npc_mounteadialogueparticipant "/Game/Blueprint/DialogueSystem/Dialogues/Via/Wagon01/MDT_Via_Wagon01.MDT_Via_Wagon01")
                (bind _asbp_dialog_main_character_3 (cast `/Game/Characters/MainCharacter/BP_DialogMainCharacter` (`GameplayStatics.GetPlayerCharacter` 0)))
                (`/MounteaDialogueSystem/Blueprints/Core/BP_Dialogue_Character.Start Dialogue from Player` _asbp_dialog_main_character_3 self)))))))))

(fn `UserConstructionScript`)