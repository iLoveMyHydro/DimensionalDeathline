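; Dialogue actor for the NPC Boob, using Mountea Dialogue to start conversations with the player character.
; StartDialogue runs only where cosmetic events can execute and a dialogue participant component exists.
; A sequence first starts a one-time conversation, tracked by a flag in BP_GameInstance.
; It then checks the GameInstance inventory for a specific item and, if present, sets the dialogue graph and starts dialogue, independent of that flag.
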(event `/Game/Blueprint/DialogueSystem/Blueprints/BPI_Dialogue.StartDialogue`
  (`/Engine/EditorBlueprintResources/StandardMacros.Can Execute Cosmetic Events`
    (:`True`
      (`/Engine/EditorBlueprintResources/StandardMacros.IsValid` (`self.GetComponentByClass` "/Script/MounteaDialogueSystem.MounteaDialogueParticipant")
        (:`Is Valid`
          (`|ExecutionSequence`
            (:`then_0`
              (bind _asbp_game_instance (cast `/Game/Blueprint/GameInstance/BP_GameInstance` (`GameplayStatics.GetGameInstance`)))
              (if (not (`/Game/Blueprint/GameInstance/BP_GameInstance.b_TalkedWithBoob` _asbp_game_instance))
                (bind _asbp_dialog_main_character (cast `/Game/Characters/MainCharacter/BP_DialogMainCharacter` (`GameplayStatics.GetPlayerCharacter` 0)))
                (`/MounteaDialogueSystem/Blueprints/Core/BP_Dialogue_Character.Start Dialogue from Player` _asbp_dialog_main_character self)
                (bind _asbp_game_instance_2 (cast `/Game/Blueprint/GameInstance/BP_GameInstance` (`GameplayStatics.GetGameInstance`)))
                (set `/Game/Blueprint/GameInstance/BP_GameInstance.b_TalkedWithBoob` true _asbp_game_instance_2)))
            (:`then_1`
              (bind _asbp_game_instance_3 (cast `/Game/Blueprint/GameInstance/BP_GameInstance` (`GameplayStatics.GetGameInstance`)))
              (if (`KismetArrayLibrary.Array_Contains` (`/Game/Blueprint/GameInstance/BP_GameInstance.Inventory` _asbp_game_instance_3) "NewEnumerator0")
                (`MounteaDialogueParticipantInterface.SetDialogueGraph` (`self.NPC_MounteaDialogueParticipant`) null)
                (bind _asbp_dialog_main_character_2 (cast `/Game/Characters/MainCharacter/BP_DialogMainCharacter` (`GameplayStatics.GetPlayerCharacter` 0)))
                (`/MounteaDialogueSystem/Blueprints/Core/BP_Dialogue_Character.Start Dialogue from Player` _asbp_dialog_main_character_2 self)))))))))

(fn `UserConstructionScript`)