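; BP_DialogActorZaq is the dialogue actor for Zaq, starting a one-time conversation with the player through the Mountea dialogue system.
; StartDialogue checks cosmetic-event execution and the participant component, then has BP_DialogMainCharacter start dialogue with this actor if the GameInstance's talked-with-Zaq flag is unset.
; It then sets that flag, blocking repeat conversations.
; An unconnected, inventory-gated branch for switching dialogue graphs never runs.
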(event `/Game/Blueprint/DialogueSystem/Blueprints/BPI_Dialogue.StartDialogue`
  (`/Engine/EditorBlueprintResources/StandardMacros.Can Execute Cosmetic Events`
    (:`True`
      (`/Engine/EditorBlueprintResources/StandardMacros.IsValid` (`self.GetComponentByClass` "/Script/MounteaDialogueSystem.MounteaDialogueParticipant")
        (:`Is Valid`
          (`|ExecutionSequence`
            (:`then_0`
              (bind _asbp_game_instance (cast `/Game/Blueprint/GameInstance/BP_GameInstance` (`GameplayStatics.GetGameInstance`)))
              (if (not (`/Game/Blueprint/GameInstance/BP_GameInstance.b_TalkedWithZaq` _asbp_game_instance))
                (bind _asbp_dialog_main_character (cast `/Game/Characters/MainCharacter/BP_DialogMainCharacter` (`GameplayStatics.GetPlayerCharacter` 0)))
                (`/MounteaDialogueSystem/Blueprints/Core/BP_Dialogue_Character.Start Dialogue from Player` _asbp_dialog_main_character self)
                (bind _asbp_game_instance_2 (cast `/Game/Blueprint/GameInstance/BP_GameInstance` (`GameplayStatics.GetGameInstance`)))
                (set `/Game/Blueprint/GameInstance/BP_GameInstance.b_TalkedWithZaq` true _asbp_game_instance_2)))))))))

(fn `UserConstructionScript`)