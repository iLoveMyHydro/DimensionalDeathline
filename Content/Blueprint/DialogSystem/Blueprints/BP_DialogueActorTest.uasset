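; BP_DialogueActorTest is a test actor the player can talk to through the Mountea dialogue system.
; LookAt returns a talk prompt, and Interact switches the first player controller to UI-only input focused on the dialog widget.
; When cosmetic events can execute and the actor has a dialogue participant component, it asks BP_DialogMainCharacter to start the dialogue, passing itself.
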(event `/Game/Blueprint/InteractableSystem/BPI_Interactable.Interact`
  (`WidgetBlueprintLibrary.SetInputMode_UIOnlyEx` (`GameplayStatics.GetPlayerController` 0) (`self.wbp_Dialog`))
  (`/Engine/EditorBlueprintResources/StandardMacros.Can Execute Cosmetic Events`
    (:`True`
      (`/Engine/EditorBlueprintResources/StandardMacros.IsValid` (`self.GetComponentByClass` "/Script/MounteaDialogueSystem.MounteaDialogueParticipant")
        (:`Is Valid`
          (bind _asbp_dialog_main_character (cast `/Game/Characters/MainCharacter/BP_DialogMainCharacter` (`GameplayStatics.GetPlayerCharacter` 0)))
          (`/MounteaDialogueSystem/Blueprints/Core/BP_Dialogue_Character.Start Dialogue from Player` _asbp_dialog_main_character self))))))

(fn `LookAt`
  (returns (t_Message :type Text))
  (return "Press E to Talk"))

(fn `UserConstructionScript`)