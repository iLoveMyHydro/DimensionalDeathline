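; Actor component that lets the player detect and interact with the object in view.
; Each tick, a short-radius sphere trace runs forward from the player camera, ignoring the owner, and caches the hit actor, clearing it on a miss.
; A newly targeted actor's look-at message is printed as debug text.
; The IA_Interact input calls InteractMessage on the cached actor if it implements BPI_Interactable.
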(event `self.ReceiveTick`
  (params (DeltaSeconds :type "Float (single-precision)"))
  (`self.InteractionTrace`))

(event `EnhancedInput|/Game/Characters/MainCharacter/Input/Actions/IA_Interact`
  (params (ActionValue :type Boolean) (ElapsedSeconds :type "Float (double-precision)") (TriggeredSeconds :type "Float (double-precision)") (InputAction :type "InputAction Object Reference" :default "/Game/Characters/MainCharacter/Input/Actions/IA_Interact.IA_Interact"))
  (:`Started`
    (bind _a_lookatactor (`self.a_LookAtActor`)
      (:`then`
        (if (`KismetSystemLibrary.DoesImplementInterface` _a_lookatactor "/Game/Blueprint/InteractableSystem/BPI_Interactable.BPI_Interactable_C")
          (message `/Game/Blueprint/InteractableSystem/BPI_Interactable.Interact` _a_lookatactor)))
      (:`else`))))

(fn `InteractionTrace`
  (bind _returnvalue (`GameplayStatics.GetPlayerCameraManager` 0))
  (bind _returnvalue_2 (`Actor.K2_GetActorLocation` _returnvalue))
  (bind (_outhit _returnvalue_3) (`KismetSystemLibrary.SphereTraceSingle` _returnvalue_2 (+ _returnvalue_2 (* (`Actor.GetActorForwardVector` _returnvalue) (`self.f_InteractionRange`))) 15.0 "TraceTypeQuery3" false (`|MakeArray` (`self.GetOwner`))))
  (if _returnvalue_3
    (bind (_bblockinghit _binitialoverlap _time _distance _location _impactpoint _normal _impactnormal _physmat _hitactor) (`GameplayStatics.BreakHitResult` _outhit))
    (if (!= _hitactor (`self.a_LookAtActor`))
      (bind _output_get (set `self.a_LookAtActor` _hitactor))
      (bind _t_message (message `/Game/Blueprint/InteractableSystem/BPI_Interactable.LookAt` _output_get))
      (`KismetSystemLibrary.PrintString` (`KismetTextLibrary.Conv_TextToString` _t_message)))
    (else
      (set `self.a_LookAtActor` null))))