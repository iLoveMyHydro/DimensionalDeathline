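; BP_jukebox is an interactable jukebox in the inventory system's items that toggles its audio playback.
; Interactwith checks whether Audio1 is playing, then stops it or starts it from the beginning.
; LookAt returns an empty string, and BeginPlay and the construction script do nothing.
; An unconnected stop, delay and replay chain remains in the event graph but never runs.
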(event `self.InteractWith`
  (bind _audio1 (`self.Audio1`))
  (if (`AudioComponent.IsPlaying` (`self.Audio1`))
    (`AudioComponent.Stop` _audio1)
    (else
      (`AudioComponent.Play` _audio1 0.0))))

(event `self.ReceiveBeginPlay`)

(fn `LookAt`
  (returns (t_Message :type Text))
  (return ""))

(fn `UserConstructionScript`)