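; BP_DoorTest is an interactable test door in the inventory system that responds only when the player's inventory holds a specific item.
; Interactwith checks the inventory and a first-open flag, both stored in BP_GameInstance.
; The first use plays an unlock animation on the skeletal mesh and clears that shared flag, while later uses play a regular open-close animation.
; LookAt returns empty text.
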(event `/Game/Blueprint/InventorySystem/BPI_Interact.InteractWith`
  (bind _asbp_game_instance (cast `/Game/Blueprint/GameInstance/BP_GameInstance` (`GameplayStatics.GetGameInstance`)))
  (if (`KismetArrayLibrary.Array_Contains` (`/Game/Blueprint/GameInstance/BP_GameInstance.Inventory` _asbp_game_instance) "NewEnumerator8")
    (bind _asbp_game_instance_2 (cast `/Game/Blueprint/GameInstance/BP_GameInstance` (`GameplayStatics.GetGameInstance`)))
    (if (`/Game/Blueprint/GameInstance/BP_GameInstance.b_OpenDoorFirstTime` _asbp_game_instance_2)
      (`SkeletalMeshComponent.PlayAnimation` (`self.SkeletalMesh`) "/Game/Modular_Assets/Meshes/Animations/A_Door_unlock_close.A_Door_unlock_close" false)
      (bind _asbp_game_instance_3 (cast `/Game/Blueprint/GameInstance/BP_GameInstance` (`GameplayStatics.GetGameInstance`)))
      (set `/Game/Blueprint/GameInstance/BP_GameInstance.b_OpenDoorFirstTime` false _asbp_game_instance_3)
      (else
        (`SkeletalMeshComponent.PlayAnimation` (`self.SkeletalMesh`) "/Game/Modular_Assets/Meshes/Animations/Animation_Door_open_close.Animation_Door_open_close" false)
        (cast `/Game/Blueprint/GameInstance/BP_GameInstance` (`GameplayStatics.GetGameInstance`))))))

(fn `LookAt`
  (returns (t_Message :type Text))
  (return ""))

(fn `UserConstructionScript`)