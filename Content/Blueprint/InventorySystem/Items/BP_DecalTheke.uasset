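; BP_DecalTheke is an interactable clue decal showing a vandalized door the player can discover.
; On interaction it sets the found-decal-in-door flag on BP_GameInstance and plays its audio.
; It then shows a hint in the main HUD's clue system widget and hides that widget after five seconds.
; Its LookAt function returns an empty string.
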(event `self.InteractWith`
  (bind _asbp_game_instance (cast `/Game/Blueprint/GameInstance/BP_GameInstance` (`GameplayStatics.GetGameInstance`)))
  (set `/Game/Blueprint/GameInstance/BP_GameInstance.b_FoundDecalInDoor` true _asbp_game_instance)
  (`AudioComponent.Play` (`self.Audio`) 0.0)
  (bind _asbp_main_hud (cast `/Game/Characters/MainCharacter/HUD/BP_MainHUD` (`PlayerController.GetHUD` (`GameplayStatics.GetPlayerController` 0))))
  (bind _wbp_cluesystemref (`/Game/Characters/MainCharacter/HUD/BP_MainHUD.wbp_ClueSystemRef` _asbp_main_hud))
  (`TextBlock.SetText` (`/Game/UI/InGameUI/Dialogue/WBP_ClueSystem.DialogueText` _wbp_cluesystemref) "Mhhh... The door was vandalized. I should write that down.  \n(press Q to open clues)")
  (`Widget.SetVisibility` _wbp_cluesystemref "Visible")
  (`KismetSystemLibrary.Delay` 5.0)
  (`Widget.SetVisibility` _wbp_cluesystemref "Hidden"))

(fn `LookAt`
  (returns (t_Message :type Text))
  (return ""))

(fn `UserConstructionScript`)