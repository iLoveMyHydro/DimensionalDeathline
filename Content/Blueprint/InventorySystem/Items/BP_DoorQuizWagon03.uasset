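; Interactable quiz door for Wagon 03 that opens once the player solves a puzzle.
; Interacting shows the HUD's puzzle widget in UI-only input, then polls every 0.1 seconds until solved and restores game input.
; A GameInstance flag selects a one-time unlock animation or the regular open-close one.
; The star emissive in a material parameter collection starts red and turns teal after the first unlock.
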(event `self.ReceiveBeginPlay`
  (`KismetMaterialLibrary.SetVectorParameterValue` "/Game/shader/mpc/MPC_Wagon03Star.MPC_Wagon03Star" "star emissive" (make `LinearColor` 1.0 0.0 0.0 1.0)))

(event `self.InteractWith`
  (bind _returnvalue (`GameplayStatics.GetPlayerController` 0))
  (bind _returnvalue_2 (`GameplayStatics.GetPlayerController` 0))
  (bind _asbp_main_hud (cast `/Game/Characters/MainCharacter/HUD/BP_MainHUD` (`PlayerController.GetHUD` (`GameplayStatics.GetPlayerController` 0))))
  (bind _wbp_puzzlewidgetref (`/Game/Characters/MainCharacter/HUD/BP_MainHUD.wbp_PuzzleWidgetRef` _asbp_main_hud))
  (`Widget.SetVisibility` _wbp_puzzlewidgetref "Visible")
  (`WidgetBlueprintLibrary.SetInputMode_UIOnlyEx` _returnvalue null)
  (set `PlayerController.bShowMouseCursor` true _returnvalue)
  (if (`/Game/UI/InGameUI/PicturePuzzle/WBP_PuzzleWidget.b_PuzzleSolved` _wbp_puzzlewidgetref) :!label _label
    (set `PlayerController.bShowMouseCursor` false _returnvalue_2)
    (`WidgetBlueprintLibrary.SetInputMode_GameOnly` _returnvalue_2)
    (bind _asbp_game_instance (cast `/Game/Blueprint/GameInstance/BP_GameInstance` (`GameplayStatics.GetGameInstance`)))
    (if (`/Game/Blueprint/GameInstance/BP_GameInstance.b_OpenWagon03DoorFirstTime` _asbp_game_instance)
      (`SkeletalMeshComponent.PlayAnimation` (`self.SkeletalMesh`) "/Game/Modular_Assets/Meshes/Animations/Animation_Door_unlock_close.Animation_Door_unlock_close" false)
      (bind _asbp_game_instance_2 (cast `/Game/Blueprint/GameInstance/BP_GameInstance` (`GameplayStatics.GetGameInstance`)))
      (set `/Game/Blueprint/GameInstance/BP_GameInstance.b_OpenWagon03DoorFirstTime` false _asbp_game_instance_2)
      (`KismetSystemLibrary.Delay` 13.0)
      (`KismetMaterialLibrary.SetVectorParameterValue` "/Game/shader/mpc/MPC_Wagon03Star.MPC_Wagon03Star" "star emissive" (make `LinearColor` 0.0 0.08022 0.138432 1.0))
      (else
        (`SkeletalMeshComponent.PlayAnimation` (`self.SkeletalMesh`) "/Game/Modular_Assets/Meshes/Animations/Animation_Door_open_close.Animation_Door_Open_close" false)
        (cast `/Game/Blueprint/GameInstance/BP_GameInstance` (`GameplayStatics.GetGameInstance`))))
    (else
      (`KismetSystemLibrary.Delay` 0.1)
      (goto _label))))

(fn `LookAt`
  (returns (t_Message :type Text))
  (return ""))

(fn `UserConstructionScript`)