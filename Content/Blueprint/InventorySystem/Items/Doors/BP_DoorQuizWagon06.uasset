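; Quiz-locked door for Wagon 06 in the inventory/interaction system, responding only once the player holds the door star.
; Interacting reveals the star, then reads and clears the HUD puzzle widget's password flag.
; A correct first attempt plays the unlock animation and clears the GameInstance first-time flag; later interactions play the regular open-close animation.
; A material parameter collection makes the star glow red, switching to blue-teal after the delayed unlock.
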(event `self.ReceiveBeginPlay`
  (`KismetMaterialLibrary.SetVectorParameterValue` "/Game/shader/mpc/MPC_Wagon06Star.MPC_Wagon06Star" "star emissive" (make `LinearColor` 1.0 0.0 0.0 1.0)))

(event `self.InteractWith`
  (bind _asbp_game_instance (cast `/Game/Blueprint/GameInstance/BP_GameInstance` (`GameplayStatics.GetGameInstance`)))
  (if (`/Game/Blueprint/GameInstance/BP_GameInstance.b_GotDoorStar` _asbp_game_instance)
    (`SceneComponent.SetHiddenInGame` (`self.Star`) false false)
    (bind _asbp_main_hud (cast `/Game/Characters/MainCharacter/HUD/BP_MainHUD` (`PlayerController.GetHUD` (`GameplayStatics.GetPlayerController` 0))))
    (bind _output_get (set `self.WBP_DoorPuzzleRef` (`/Game/Characters/MainCharacter/HUD/BP_MainHUD.wbp_DoorPuzzleRef` _asbp_main_hud)))
    (if (`/Game/UI/InGameUI/DoorPuzzle/WBP_PuzzleMain.b_PasswordIsCorrect` _output_get)
      (set `/Game/UI/InGameUI/DoorPuzzle/WBP_PuzzleMain.b_PasswordIsCorrect` false (`self.WBP_DoorPuzzleRef`))
      (bind _asbp_game_instance_2 (cast `/Game/Blueprint/GameInstance/BP_GameInstance` (`GameplayStatics.GetGameInstance`)))
      (if (`/Game/Blueprint/GameInstance/BP_GameInstance.b_OpenWagon06DoorFirstTime` _asbp_game_instance_2)
        (`SkeletalMeshComponent.PlayAnimation` (`self.SkeletalMesh`) "/Game/Modular_Assets/Meshes/Animations/Animation_Door_unlock_close.Animation_Door_unlock_close" false)
        (bind _asbp_game_instance_3 (cast `/Game/Blueprint/GameInstance/BP_GameInstance` (`GameplayStatics.GetGameInstance`)))
        (set `/Game/Blueprint/GameInstance/BP_GameInstance.b_OpenWagon06DoorFirstTime` false _asbp_game_instance_3)
        (`KismetSystemLibrary.Delay` 13.0)
        (`KismetMaterialLibrary.SetVectorParameterValue` "/Game/shader/mpc/MPC_Wagon06Star.MPC_Wagon06Star" "star emissive" (make `LinearColor` 0.0 0.08022 0.138432 1.0))
        (else
          (`SkeletalMeshComponent.PlayAnimation` (`self.SkeletalMesh`) "/Game/Modular_Assets/Meshes/Animations/Animation_Door_open_close.Animation_Door_Open_close" false :!label _label)
          (cast `/Game/Blueprint/GameInstance/BP_GameInstance` (`GameplayStatics.GetGameInstance`))))
      (else
        (bind _asbp_game_instance_4 (cast `/Game/Blueprint/GameInstance/BP_GameInstance` (`GameplayStatics.GetGameInstance`)))
        (if (`/Game/Blueprint/GameInstance/BP_GameInstance.b_OpenWagon06DoorFirstTime` _asbp_game_instance_4)
          (set `/Game/UI/InGameUI/DoorPuzzle/WBP_PuzzleMain.b_PasswordIsCorrect` false (`self.WBP_DoorPuzzleRef`))
          (else
            (goto _label)))))))

(fn `LookAt`
  (returns (t_Message :type Text))
  (return ""))

(fn `UserConstructionScript`)