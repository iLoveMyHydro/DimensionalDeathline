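; Interactable third door button for wagon 02 that opens a password puzzle.
; Interacting freezes the player and, if unsolved, configures and shows the HUD's door puzzle widget with a hardcoded password and UI-only mouse input.
; A Delay loop polls the widget until the password is correct.
; Success plays audio, swaps symbol materials on all three wagon 02 buttons, found by class, and restores walking.
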(event `self.InteractWith`
  (bind _returnvalue (`GameplayStatics.GetPlayerController` 0))
  (bind _asbp_dialog_main_character (cast `/Game/Characters/MainCharacter/BP_DialogMainCharacter` (`GameplayStatics.GetPlayerCharacter` 0)))
  (`CharacterMovementComponent.DisableMovement` (`Character.CharacterMovement` _asbp_dialog_main_character))
  (bind _asbp_main_hud (cast `/Game/Characters/MainCharacter/HUD/BP_MainHUD` (`PlayerController.GetHUD` (`GameplayStatics.GetPlayerController` 0))))
  (bind _output_get (set `self.wbp_MainQuizRef` (`/Game/Characters/MainCharacter/HUD/BP_MainHUD.wbp_DoorPuzzleRef` _asbp_main_hud)))
  (if (not (`/Game/UI/InGameUI/DoorPuzzle/WBP_PuzzleMain.b_PasswordIsCorrect` _output_get))
    (set `/Game/UI/InGameUI/DoorPuzzle/WBP_PuzzleImage.i_MaxNumbers` 26 (`/Game/UI/InGameUI/DoorPuzzle/WBP_PuzzleMain.WBP_PuzzleImage` _output_get))
    (set `/Game/UI/InGameUI/DoorPuzzle/WBP_PuzzleImage.i_MaxNumbers` 26 (`/Game/UI/InGameUI/DoorPuzzle/WBP_PuzzleMain.WBP_PuzzleImage_3` _output_get))
    (set `/Game/UI/InGameUI/DoorPuzzle/WBP_PuzzleMain.i_Passwords` 2841 _output_get)
    (set `/Game/UI/InGameUI/DoorPuzzle/WBP_PuzzleImage.i_MaxNumbers` 26 (`/Game/UI/InGameUI/DoorPuzzle/WBP_PuzzleMain.WBP_PuzzleImage_2` _output_get))
    (`/Game/UI/InGameUI/DoorPuzzle/WBP_PuzzleMain.OnVisible` _output_get)
    (`Widget.SetVisibility` _output_get "Visible")
    (`Widget.SetVisibility` (`/Game/UI/InGameUI/DoorPuzzle/WBP_PuzzleMain.WBP_PuzzleImage` _output_get) "Visible")
    (`Widget.SetVisibility` (`/Game/UI/InGameUI/DoorPuzzle/WBP_PuzzleMain.WBP_PuzzleImage_3` _output_get) "Visible")
    (`Widget.SetVisibility` (`/Game/UI/InGameUI/DoorPuzzle/WBP_PuzzleMain.WBP_PuzzleImage_2` _output_get) "Visible")
    (set `PlayerController.bShowMouseCursor` true _returnvalue)
    (`WidgetBlueprintLibrary.SetInputMode_UIOnlyEx` _returnvalue null)
    (`KismetSystemLibrary.Delay` 0.1 :!label _label)
    (if (`/Game/UI/InGameUI/DoorPuzzle/WBP_PuzzleMain.b_PasswordIsCorrect` (`self.wbp_MainQuizRef`))
      (`AudioComponent.Play` (`self.Audio`) 0.0)
      (`PrimitiveComponent.SetMaterial` (`self.Button`) 1 "/Game/Environment_Assets/Symbole/MI_Symbol_Wagon02Finished3.MI_Symbol_Wagon02Finished3")
      (bind _returnvalue_2 (`GameplayStatics.GetActorOfClass` "/Game/Blueprint/InventorySystem/Items/DoorButton/BP_DoorButtonWagon02_1.BP_DoorButtonWagon02_1_C"))
      (`PrimitiveComponent.SetMaterial` (`/Game/Blueprint/InventorySystem/Items/DoorButton/BP_DoorButtonWagon02_1.Button` _returnvalue_2) 1 "/Game/Environment_Assets/Symbole/MI_Symbol_Wagon02Finished1.MI_Symbol_Wagon02Finished1")
      (bind _returnvalue_3 (`GameplayStatics.GetActorOfClass` "/Game/Blueprint/InventorySystem/Items/DoorButton/BP_DoorButtonWagon02_2.BP_DoorButtonWagon02_2_C"))
      (`PrimitiveComponent.SetMaterial` (`/Game/Blueprint/InventorySystem/Items/DoorButton/BP_DoorButtonWagon02_2.Button` _returnvalue_3) 1 "/Game/Environment_Assets/Symbole/MI_Symbol_Wagon02Finished2.MI_Symbol_Wagon02Finished2")
      (bind _asbp_dialog_main_character_2 (cast `/Game/Characters/MainCharacter/BP_DialogMainCharacter` (`GameplayStatics.GetPlayerCharacter` 0)))
      (`CharacterMovementComponent.SetMovementMode` (`Character.CharacterMovement` _asbp_dialog_main_character_2) "MOVE_Walking" 0)
      (else
        (goto _label)))))

(fn `LookAt`
  (returns (t_Message :type Text))
  (return ""))

(fn `UserConstructionScript`)