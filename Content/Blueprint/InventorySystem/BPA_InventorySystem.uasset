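; Inventory component that holds a fixed-size slot array and handles the owner's item interaction.
; A per-tick camera sphere trace tracks the looked-at actor, and the Interact input messages its BPA_ItemDataComponent.
; AddToInventory places items one at a time into matching stacks, capped by DT_ItemData stack sizes, or into empty slots, returning any remainder.
; RemoveFromInventory is an empty stub, and key 1 prints the contents for debugging.
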(event `self.ReceiveBeginPlay`
  (`KismetArrayLibrary.Array_Resize` (`self.s_Content`) (`self.i_InventorySize`)))

(event `self.ReceiveTick`
  (params (DeltaSeconds :type "Float (single-precision)"))
  (`self.InteractionTrace`))

(event `EnhancedInput|/Game/Characters/MainCharacter/Input/Actions/IA_Interact`
  (params (ActionValue :type Boolean) (ElapsedSeconds :type "Float (double-precision)") (TriggeredSeconds :type "Float (double-precision)") (InputAction :type "InputAction Object Reference" :default "/Game/Characters/MainCharacter/Input/Actions/IA_Interact.IA_Interact"))
  (:`Triggered`
    (bind _a_lookatactor (`self.a_LookAtActor`)
      (:`then`
        (bind _returnvalue (`Actor.GetComponentByClass` _a_lookatactor "/Game/Blueprint/InventorySystem/BPA_ItemDataComponent.BPA_ItemDataComponent_C"))
        (`/Engine/EditorBlueprintResources/StandardMacros.IsValid` _returnvalue
          (:`Is Valid`
            (message `/Game/Blueprint/InventorySystem/BPI_Interact.InteractWith` _returnvalue (cast `/Game/Characters/MainCharacter/BP_DialogMainCharacter` (`self.GetOwner`) :!pure true)))))
      (:`else`))))

(event `Key|One`
  (params (Key :type "Key Structure"))
  (:`Pressed`
    (`self.DEBUG_PRINTCONTENTS`)))

(fn `AddToInventory`
  (params (n_ItemID :type Name) (i_Quantity :type Integer))
  (returns (b_Sucess :type Boolean) (i_QuantityRemaining :type Integer))
  (locals (i_LocalQuantityRemaining :type Integer) (b_LocalHasFailed :type Boolean))
  (set `local.i_LocalQuantityRemaining` i_Quantity)
  (while (and (> (`local.i_LocalQuantityRemaining`) 0) (not (`local.b_LocalHasFailed`)))
    (bind (_i_index _b_foundslot) (`self.FindSlot` (`local.n_ItemID`)))
    (if _b_foundslot
      (`self.AddToStack` _i_index 1)
      (`/Engine/EditorBlueprintResources/StandardMacros.DecrementInt` (`local.i_LocalQuantityRemaining`))
      (elif (`self.AnyEmptySlotsAvailable`)
        (bind _b_success (`self.CreateNewStack` (`local.n_ItemID`) 1))
        (if _b_success
          (`/Engine/EditorBlueprintResources/StandardMacros.DecrementInt` (`local.i_LocalQuantityRemaining`))
          (else
            (set `local.b_LocalHasFailed` true)))
        (else
          (set `local.b_LocalHasFailed` true)))))
  (return (not (`local.b_LocalHasFailed`)) (`local.i_LocalQuantityRemaining`)))

(fn `AddToStack`
  (params (i_Index :type Integer) (i_Quantity :type Integer))
  (bind _s_content (`self.s_Content`))
  (bind (_output_itemid _output_quantity) (break `/Game/Blueprint/InventorySystem/FSlotStruct` (`|GetArrayItem` _s_content i_Quantity)))
  (`KismetArrayLibrary.Array_Set` _s_content i_Index (make `/Game/Blueprint/InventorySystem/FSlotStruct` _output_itemid (+ _output_quantity (`local.i_Quantity`)))))

(fn `AnyEmptySlotsAvailable`
  (returns (b_HasEmptySlot :type Boolean) (i_EmptyIndex :type Integer))
  (for (_array_element _array_index) (`self.s_Content`)
    (if (== (`.Quantity_5_BF6C18F8494C8F4F25F9AC8994707A79` (break `/Game/Blueprint/InventorySystem/FSlotStruct` _array_element)) 0)
      (return true _array_index)))
  (return false -1))

(fn `CreateNewStack`
  (params (n_ItemID :type Name) (i_Quantity :type Integer))
  (returns (b_Success :type Boolean))
  (bind (_b_hasemptyslot _i_emptyindex) (`self.AnyEmptySlotsAvailable`))
  (if _b_hasemptyslot
    (`KismetArrayLibrary.Array_Set` (`self.s_Content`) _i_emptyindex (make `/Game/Blueprint/InventorySystem/FSlotStruct` n_ItemID i_Quantity))
    (return true)
    (else
      (return false))))

(fn `DEBUG_PRINTCONTENTS`
  (for (_array_element _array_index) (`self.s_Content`)
    (bind (_itemid _quantity) (break `/Game/Blueprint/InventorySystem/FSlotStruct` _array_element))
    (`KismetSystemLibrary.PrintString` (`KismetStringLibrary.Concat_StrStr` (`KismetStringLibrary.Conv_IntToString` _array_index) "  " (`KismetStringLibrary.Conv_NameToString` _itemid) " = " (`KismetStringLibrary.Conv_IntToString` _quantity)))))

(fn `FindSlot`
  (params (n_ItemID :type Name))
  (returns (i_Index :type Integer) (b_FoundSlot :type Boolean))
  (for (_array_element _array_index) (`self.s_Content`)
    (bind (_itemid _quantity) (break `/Game/Blueprint/InventorySystem/FSlotStruct` _array_element))
    (if (== _itemid n_ItemID)
      (if (< _quantity (`self.GetMaxStackSIze` n_ItemID))
        (return _array_index true))))
  (return -1 false))

(fn `GetMaxStackSIze`
  (params (n_ItemID :type Name))
  (returns (`Out Row Stack Size` :type Integer))
  (bind _returnvalue (`|GetDataTableRow` "/Game/Blueprint/InventorySystem/DT_ItemData.DT_ItemData" n_ItemID)
    (:`then`
      (return (`.StackSize_14_F7E229314BB1179BA2C869B6E8D57F65` (break `/Game/Blueprint/InventorySystem/FItemStruct` _returnvalue))))
    (:`RowNotFound`
      (return -1))))

(fn `InteractionTrace`
  (bind _returnvalue (`GameplayStatics.GetPlayerCameraManager` 0))
  (bind _returnvalue_2 (`Actor.K2_GetActorLocation` _returnvalue))
  (bind (_outhit _returnvalue_3) (`KismetSystemLibrary.SphereTraceSingle` _returnvalue_2 (+ _returnvalue_2 (* (`Actor.GetActorForwardVector` _returnvalue) (`self.f_InteractionRange`))) 15.0 "TraceTypeQuery3" false (`|MakeArray` (`self.GetOwner`))))
  (if _returnvalue_3
    (bind (_bblockinghit _binitialoverlap _time _distance _location _impactpoint _normal _impactnormal _physmat _hitactor) (`GameplayStatics.BreakHitResult` _outhit))
    (if (!= _hitactor (`self.a_LookAtActor`))
      (bind _output_get (set `self.a_LookAtActor` _hitactor))
      (bind _t_message (message `/Game/Blueprint/InventorySystem/BPI_Interact.LookAt` _output_get))
      (`KismetSystemLibrary.PrintString` (`KismetTextLibrary.Conv_TextToString` _t_message)))
    (else
      (set `self.a_LookAtActor` null))))

(fn `RemoveFromInventory`)