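; BP_cutscene is an actor that plays a timed video cutscene, then loads MainLevel.
; On BeginPlay it adds a WBP_video widget to the viewport, adds two audio components, switches to UI-only input and hides the cursor.
; After a fixed delay it removes the widget, calls DestroyActor on itself, restores game-only input and opens the level by name.
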(event `self.ReceiveBeginPlay`
  (bind _returnvalue (`GameplayStatics.GetPlayerController` 0))
  (bind _returnvalue_2 (`|CreateWidget` "/Game/VFX/WBP_video.WBP_video_C"))
  (`AddComponent|NODE_AddAudioComponent-1`)
  (`UserWidget.AddToViewport` _returnvalue_2 0)
  (`AddComponent|NODE_AddAudioComponent-0`)
  (`WidgetBlueprintLibrary.SetInputMode_UIOnlyEx` (`GameplayStatics.GetPlayerController` 0) null)
  (set `PlayerController.bShowMouseCursor` false _returnvalue)
  (`KismetSystemLibrary.Delay` 27.0)
  (`Widget.RemoveFromParent` _returnvalue_2)
  (`self.K2_DestroyActor`)
  (`WidgetBlueprintLibrary.SetInputMode_GameOnly` _returnvalue)
  (`GameplayStatics.OpenLevel` "MainLevel"))

(fn `UserConstructionScript`)